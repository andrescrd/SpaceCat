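; Player controller that spawns a group of characters and moves them all at once from a single set of input axes.
; On BeginPlay, if CanSpawn is set, it spawns a BP_SCharacter and another BP_SPlayerController at every TargetPoint, storing both and having each new controller possess its character.
; Spawned controllers get CanSpawn off, preventing recursive spawning.
; Forward and Horizontal input applies movement to every stored character along its own forward and right vectors.
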(event EventBeginPlay
  (if (Variables|Default|GetbCanSpawn)
    (bind _outactors (Actor|GetAllActorsOfClass "/Script/Engine.TargetPoint"))
    (for (_ _array_index) _outactors
      (bind _returnvalue (Game|SpawnActorfromClass "/Game/Blueprints/BP_SCharacter.BP_SCharacter_C" (Math|Conversions|ToTransform(Vector) (Transformation|GetActorLocation (Utilities|Array|Get(acopy) _outactors _array_index))) "Undefined" 0 0))
      (Utilities|Array|Add (Variables|Default|GetChar) _returnvalue)
      (bind _returnvalue_2 (Game|SpawnActorfromClass "BP_SPlayerController_C" (Math|Conversions|ToTransform(Vector) (Transformation|GetActorLocation (Utilities|Array|Get(acopy) _outactors _array_index))) "Undefined" 0 false 0))
      (Utilities|Array|Add (Variables|Default|GetControllers) _returnvalue_2)
      (Pawn|Possess _returnvalue_2 _returnvalue))))

(event Input|AxisEvents|InputAxisForward
  (params (AxisValue :type Float%20%28single-precision%29))
  (for _array_element (Variables|Default|GetChar)
    (Pawn|Input|AddMovementInput _array_element (Transformation|GetActorForwardVector _array_element) AxisValue false)))

(event Input|AxisEvents|InputAxisHorizontal
  (params (AxisValue :type Float%20%28single-precision%29))
  (for _array_element (Variables|Default|GetChar)
    (Pawn|Input|AddMovementInput _array_element (Transformation|GetActorRightVector _array_element) AxisValue false)))

(fn ConstructionScript)