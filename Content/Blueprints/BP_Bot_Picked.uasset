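; BP_Bot_Picked is a bot that characters can pick up, carry and drop.
; Activate prints a red "Help me" message with the activator's display name.
; Picked disables static mesh collision and attaches the bot to the Character's mesh at PickerSocket, snapping location but keeping relative rotation and scale.
; Drop detaches it, keeping world location, and restores query and physics collision.
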(event EventActivate
  (params (Activator :type Actor%20Object%20Reference))
  (Development|PrintString (Utilities|String|ToString(Text) (Utilities|Text|FormatText "Help me {0}" (Utilities|Text|ToText(String) (Utilities|GetDisplayName Activator)))) true true "(R=1.000000,G=0.005931,B=0.000000,A=1.000000)"))

(event EventPicked
  (params (CurrentActor :type Actor%20Object%20Reference))
  ;[0.564 0 1] Actor is Picked
  (Collision|SetCollisionEnabled (Variables|Debug|GetStaticMeshComponent) "NoCollision")
  (Transformation|AttachComponentToComponent (Variables|/Script/Engine.Character|GetMesh (.AsCharacter (Utilities|Casting|CastToCharacter CurrentActor))) "PickerSocket" "SnapToTarget" "KeepRelative" "KeepRelative" true))

(event EventDrop
  (params (CurrentActor :type Actor%20Object%20Reference))
  ;[1 0.1033 0] Actor is Dropped
  (Transformation|DetachFromActor "KeepWorld" "KeepRelative" "KeepRelative")
  (Collision|SetCollisionEnabled (Variables|Debug|GetStaticMeshComponent) "QueryAndPhysics"))

(fn ConstructionScript)